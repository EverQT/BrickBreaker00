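; Speed power-up actor that temporarily changes the player character's walk speed for as long as it exists.
; On BeginPlay it stores player 0's current max movement speed, sets MaxWalkSpeed to its MaxSpeed variable and gives itself a 20-second lifespan.
; The Destroyed event writes the stored speed back to MaxWalkSpeed, without the validity checks used on BeginPlay, so the actor's lifetime acts as the effect timer.
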(event EventBeginPlay
  (bind _returnvalue (Game|GetPlayerCharacter 0))
  (bind _returnvalue_2 (Actor|GetComponentbyClass _returnvalue "/Script/Engine.CharacterMovementComponent"))
  (Utilities|IsValid _returnvalue
    (:Is%20Valid
      (Utilities|IsValid _returnvalue_2
        (:Is%20Valid
          (Variables|Default|SetInitialSpeed (Class|MovementComponent|GetMaxSpeed _returnvalue_2))
          (Variables|/Script/Engine.CharacterMovementComponent|SetMaxWalkSpeed _returnvalue_2 (Variables|Default|GetMaxSpeed))
          (Actor|SetLifeSpan 2e+01))))))

(event EventDestroyed
  (Variables|/Script/Engine.CharacterMovementComponent|SetMaxWalkSpeed (Actor|GetComponentbyClass (Game|GetPlayerCharacter 0) "/Script/Engine.CharacterMovementComponent") (Variables|Default|GetInitialSpeed)))

(fn ConstructionScript)